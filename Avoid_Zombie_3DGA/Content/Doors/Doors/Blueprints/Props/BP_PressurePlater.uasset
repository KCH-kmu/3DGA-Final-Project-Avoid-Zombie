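; Pressure plate prop that sinks when the player steps on it and fires an OnPlateDown dispatcher, intended to unlock doors, once fully down.
; Box overlaps play or reverse a timeline, so leaving early raises the plate, while a fully pressed plate stays down.
; Each update lerps Z from the plate's current location toward a small directional offset, so movement is incremental rather than between fixed endpoints.
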(event OnComponentBeginOverlap(Box)
  (params (OverlappedComponent :type Primitive%20Component%20Object%20Reference) (OtherActor :type Actor%20Object%20Reference) (OtherComp :type Primitive%20Component%20Object%20Reference) (OtherBodyIndex :type Integer) (bFromSweep :type Boolean) (SweepResult :type Hit%20Result%20Structure%20%28by%20ref%29))
  ;[1 1 1] If the player is standing on pressure plate go down
  (if (== OtherActor (Game|GetPlayerCharacter 0))
    (Audio|Components|Audio|Play (Variables|Default|GetActivatePressurePlate))))

(event OnComponentEndOverlap(Box)
  (params (OverlappedComponent :type Primitive%20Component%20Object%20Reference) (OtherActor :type Actor%20Object%20Reference) (OtherComp :type Primitive%20Component%20Object%20Reference) (OtherBodyIndex :type Integer))
  ;[1 1 1] If the player is off the pressure plate and the plate rises if it wasnt fully down
  (if (and (== OtherActor (Game|GetPlayerCharacter 0)) (not (Variables|Default|GetFullyDown)))
    (Utilities|String|Reverse (Variables|Default|GetActivatePressurePlate))))

(fn ConstructionScript)