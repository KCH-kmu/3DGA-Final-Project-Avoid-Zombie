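; Interactive physics door that the player opens, kicks or knocks on, based on lock state, movement speed and destructibility; destroying its Key actor unlocks it.
; Interact walks and rotates the player to an arrow, then plays a motion-warped montage whose notifies open or destroy it.
; Opening runs a timeline before re-enabling physics, while a trigger-box timer polls swing velocity for creak and slam sounds.
; Kicks or damage shatter destroyable doors through Chaos fields.
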(event OnComponentBeginOverlap(Box)
  (params (OverlappedComponent :type Primitive%20Component%20Object%20Reference) (OtherActor :type Actor%20Object%20Reference) (OtherComp :type Primitive%20Component%20Object%20Reference) (OtherBodyIndex :type Integer) (bFromSweep :type Boolean) (SweepResult :type Hit%20Result%20Structure%20%28by%20ref%29))
  ;[1 1 1] Physics SFX s
  ;;[1 0.852 0.05864] Start the sfx timer event if the player overlaps trigger box
  (if (== OtherActor (Game|GetPlayerCharacter 0))
    (CallFunction|PlaySfx)))

(event OnComponentEndOverlap(Box)
  (params (OverlappedComponent :type Primitive%20Component%20Object%20Reference) (OtherActor :type Actor%20Object%20Reference) (OtherComp :type Primitive%20Component%20Object%20Reference) (OtherBodyIndex :type Integer))
  ;[1 1 1] Physics SFX s
  ;;[1 0.7895 0.05682] Stops the sfx loop timer when left box
  (if (== OtherActor (Game|GetPlayerCharacter 0))
    (Utilities|Time|ClearandInvalidateTimerbyHandle (Variables|Default|GetSfxTimer))
    (CallFunction|Closegate)))

(event Custom|OpenDoor
  ;[1 1 1] Timeline and sfx for door opening with no physics
  (CallFunction|ReverseTimelineReset)
  ;;[1 1 1] Sets the door to be open or closed depending on status
  (bind (_direction _rotationtimeline) (Timeline|DoorOpening Play)
    (:Update
      (Transformation|SetRelativeRotation (Variables|Default|GetDoorMiddle) (Math|Rotator|MakeRotator 0.0 0.0 (Math|Float|Lerp 0.0 -9e+01 _rotationtimeline)) false false)
      ;;[1 1 1] stops the physics so physics dont interupt the timeline plays the creek sfx sound
      (Physics|SetSimulatePhysics (Variables|Default|GetDoorMiddle) false)
      (Utilities|FlowControl|DoOnce false
        (:Completed
          (CallFunction|SpawnSFX (Variables|Default|GetCreekSound) (Variables|Default|GetFrame)))))
    (:Finished
      (Variables|Default|SetDoorOpen (Utilities|Enum|Equal(Enum) _direction "Forward"))
      ;;[1 1 1] Plays the door slamming sound sfx then sets the physics so door swings back
      (CallFunction|SpawnSFX (Variables|Default|GetDoorSlammingSound) (Variables|Default|GetFrame))
      (Utilities|FlowControl|Delay 1.0)
      ;;[1 1 1] sets door middle physics and resets the creek sfx
      (Physics|SetSimulatePhysics (Variables|Default|GetDoorMiddle) true)
      (CallFunction|ResetTimelineCreekSound)
      (Utilities|FlowControl|DoOnce false
        (:Completed
          (Utilities|String|Reverse (Variables|Default|GetDoorOpening)))))))

(event Custom|ChangeLockedDoor
  (params (DestroyedActor :type Actor%20Object%20Reference))
  ;[1 0.7042 0.6885 1 101] Begin Play
  ;;[1 1 1] Binds a event to the key variabel when key is picked up and destroyed changes the door to be unlocked
  (Variables|Default|SetDoorLocked false))

(event Custom|ResetTimelineCreekSound
  ;[1 1 1] Timeline and sfx for door opening with no physics
  ;;[1 1 1] stops the physics so physics dont interupt the timeline plays the creek sfx sound
  (Utilities|FlowControl|DoOnce false) ; enters at Reset
)

(event Custom|ResetSlamSound
  ;[1 1 1] Physics SFX s
  ;;[1 1 1] Timer for sfx Checks
  ;;;[1 1 1] If the door has stopped moving this plays the slam sfx and closes the gate to stop repeat plays it then resets the creek sound so the sfx can be played again
  (Utilities|FlowControl|Gate true) ; enters at Open
)

(event Custom|ReverseTimelineReset
  ;[1 1 1] Timeline and sfx for door opening with no physics
  ;;[1 1 1] sets door middle physics and resets the creek sfx
  (Utilities|FlowControl|DoOnce false) ; enters at Reset
)

(event Custom|DestroyDoor
  (bind _doormiddle (Variables|Default|GetDoorMiddle))
  ;[1 0 0 1 139] Chaos destruction
  ;;[1 1 1] Sets the door middle to hidden so can make the geometry collision visible to enable chaos detsruction
  (Rendering|SetVisibility _doormiddle false false)
  (Collision|SetCollisionEnabled _doormiddle "NoCollision")
  ;;[1 1 1] Makes destruction field visible
  (Rendering|SetVisibility (Variables|Default|GetGeometryCollection) true false)
  ;;[1 1 1] Spawns the master field to destroy the door
  (bind _returnvalue (Game|SpawnActorfromClass "/Engine/EditorResources/FieldNodes/FS_MasterField.FS_MasterField_C" (Math|Transform|MakeTransform (Transformation|GetWorldLocation (Variables|Default|GetArrow)) "0, 0, 0" "1.000000,1.000000,1.000000") "Undefined" "MultiplyWithRoot" 0 0))
  (Default|CETrigger _returnvalue)
  (Variables|Default|SetDoorOpen true))

(event Custom|Move%20and%20Rotate
  (params (WarpTargetName :type Name) (MontageToPlay :type Anim%20Montage%20Object%20Reference))
  ;[0 0.2803 1 1 69] Movement and rotation
  ;;[1 1 1] Starts a timer to move and rotate the player every 0.001 second
  (bind _returnvalue (Utilities|Time|SetTimerbyEvent (delegate Custom|MovementRotateEvent) 0.01 true))
  (Variables|Default|SetMoveHandle _returnvalue))

(event Custom|MovementRotateEvent
  (bind _arrow (Variables|Default|GetArrow))
  (bind _returnvalue (Transformation|GetWorldLocation _arrow))
  ;[0 0.2803 1 1 69] Movement and rotation
  ;;[1 1 1] checks if player is in the same location as the arrow tyeh destination point with 60 as the fault tolerence
  (if (Utilities|Operators|EqualEqual (Transformation|GetActorLocation (Game|GetPlayerCharacter 0)) _returnvalue 6e+01)
    ;;[1 1 1] stops the loop and starts the rotation
    (Utilities|Time|ClearandInvalidateTimerbyHandle (Variables|Default|GetMoveHandle))
    ;;[1 1 1] Rotates to the direction of the arrow
    (bind _newtrack_0 (Timeline|RotateTimeline Play)
      (:Update
        (Transformation|SetActorRotation (Game|GetPlayerCharacter 0) (Math|Rotator|Lerp(Rotator) (Transformation|GetActorRotation (Game|GetPlayerCharacter 0)) (Variables|/Script/Engine.SceneComponent|GetRelativeRotation (Variables|Default|GetArrow)) _newtrack_0 true)))
      (:Finished
        (CallFunction|PlayMontages (stale Custom|Move%20and%20Rotate WarpTargetName) (stale Custom|Move%20and%20Rotate MontageToPlay))))
    (else
      ;;[1 1 1] If not moves the actor to the location
      (AI|Navigation|SimpleMovetoLocation (Game|GetPlayerController 0) _returnvalue))))

(event Custom|PlayMontages
  (params (WarpTargetName :type Name) (MontageToPlay :type Anim%20Montage%20Object%20Reference))
  (bind _banginganim (Variables|Default|GetBangingAnim))
  ;[0.0528 0.09394 1 1 101] Play Montages
  ;;[1 1 1] Plays the montage on the character
  (bind _notifyname (Animation|Montage|PlayMontage (Actor|GetComponentbyClass (Game|GetPlayerCharacter 0) "/Script/Engine.SkeletalMeshComponent") MontageToPlay)
    (:then
      ;;[1 1 1] Motion warps over to the anim which is the reference for the animations
      (Class|MotionWarpingComponent|AddorUpdateWarpTargetfromLocationandRotation (Actor|GetComponentbyClass (Game|GetPlayerCharacter 0) "/Script/MotionWarping.MotionWarpingComponent") WarpTargetName (Transformation|GetWorldLocation _banginganim) (Transformation|GetWorldRotation _banginganim)))
    (:OnNotifyBegin
      ;;[1 1 1] If the notify inside the montages is kick or open trigger different events
      (switch name _notifyname
        (:Kick
          (if (Variables|Default|GetDestroyable)
            (CallFunction|DestroyDoor)
            (else
              (CallFunction|OpenDoor :!label _label))))
        (:Open
          (goto _label))))))

(event Custom|PlaySfx
  ;[1 1 1] Physics SFX s
  ;;[1 1 1] Timer for sfx Checks
  (bind _returnvalue (Utilities|Time|SetTimerbyEvent (delegate Custom|LoopForSFXChecks) 0.01 true))
  (Variables|Default|SetSfxTimer _returnvalue))

(event Custom|LoopForSFXChecks
  (bind _doormiddle (Variables|Default|GetDoorMiddle))
  (bind _returnvalue (Physics|GetPhysicsAngularVelocityinDegrees _doormiddle "None"))
  ;[1 1 1] Physics SFX s
  ;;[1 1 1] Timer for sfx Checks
  ;;;[1 1 1] If the door has stopped moving this plays the slam sfx and closes the gate to stop repeat plays it then resets the creek sound so the sfx can be played again
  (if (Math|Float|NearlyEqual(Float) (.z (Physics|GetPhysicsAngularVelocityinDegrees (Variables|Default|GetDoorMiddle) "None")) 0.0 5.0)
    (Utilities|FlowControl|Gate true
      (:Exit
        (CallFunction|SpawnSFX (Variables|Default|GetDoorSlammingSound) (Variables|Default|GetFrame))
        (CallFunction|Closegate)
        (goto _label Reset)))
    (else
      ;;;[1 1 1] Resets the slam sound if the door is moving and plays the creek sound once
      (if (or (> (.z _returnvalue) 1e+01) (< (.z _returnvalue) -1e+01))
        (CallFunction|ResetSlamSound)
        (Utilities|FlowControl|DoOnce false :!label _label
          (:Completed
            (CallFunction|SpawnSFX (Variables|Default|GetCreekSound) (Variables|Default|GetDoorMiddle))))))))

(event Custom|Closegate
  ;[1 1 1] Physics SFX s
  ;;[1 1 1] Timer for sfx Checks
  ;;;[1 1 1] If the door has stopped moving this plays the slam sfx and closes the gate to stop repeat plays it then resets the creek sound so the sfx can be played again
  (Utilities|FlowControl|Gate true) ; enters at Close
)

(event EventInteract
  (bind _returnvalue (Game|GetPlayerCharacter 0))
  (bind _returnvalue_2 (Actor|GetComponentbyClass _returnvalue "/Script/Engine.CharacterMovementComponent"))
  (bind _maxwalkspeed (Variables|/Script/Engine.CharacterMovementComponent|GetMaxWalkSpeed _returnvalue_2))
  (bind _returnvalue_3 (>= _maxwalkspeed 8e+02))
  ;[1 0 0.4619 1 120] Interact BPI
  ;;[1 1 1] On interact checks if door is locked
  (if (not (Variables|Default|GetDoorLocked))
    ;;[1 1 1] If door is locked checks if door has been opened already
    (if (not (Variables|Default|GetDoorOpen))
      (if _returnvalue_3
        ;;[1 1 1] Start to move and rotate player to the door needsa nav mesh around the door for player to move to
        ;;;[1 1 1] If running fast at door kick it down or if door locked and is destroyable also kick it down
        (CallFunction|MoveandRotate "Kick" "/Game/Doors/Doors/Animations/AM_SpartanKickV2_Montage.AM_SpartanKickV2_Montage" :!label _label)
        (else
          ;;;[1 1 1] If max walk speed is normal run play door open animation
          (CallFunction|MoveandRotate "Open" "/Game/Doors/Doors/Animations/AM_Vend_Start_Montage.AM_Vend_Start_Montage"))))
    (else
      ;;[1 1 1] Checks if door is destroyable
      (if (and (Variables|Default|GetDestroyable) _returnvalue_3)
        (goto _label)
        (else
          ;;;[1 1 1] bash on door if door is not detroyable and is locked
          (CallFunction|MoveandRotate "Knock" "/Game/Doors/Doors/Animations/AM_Vend_Fail_HitMachine_Montage.AM_Vend_Fail_HitMachine_Montage"))))))

(event EventBeginPlay
  ;[1 0.7042 0.6885 1 101] Begin Play
  ;;[1 1 1] Binds a event to the key variabel when key is picked up and destroyed changes the door to be unlocked
  (bind _key (Variables|Default|GetKey)
    (:then
      (Game|BindEventtoOnDestroyed _key (delegate Custom|ChangeLockedDoor)))
    (:else
      _))
  ;;[1 1 1] If door is not locked sets physics to be active creating a physics door
  (Physics|SetSimulatePhysics (Variables|Default|GetDoorMiddle) (not (Variables|Default|GetDoorLocked))))

(event Game|Damage|EventAnyDamage
  (params (Damage :type Float%20%28single-precision%29) (DamageType :type Damage%20Type%20Object%20Reference) (InstigatedBy :type Controller%20Object%20Reference) (DamageCauser :type Actor%20Object%20Reference))
  ;[1 0.1328 0.07511 1 95] Damage Event
  ;;[1 1 1] If the door takes damage spawns the master field to destroy the door allowing weapons to hit the door and destroy it
  (if (Variables|Default|GetDestroyable)
    (CallFunction|DestroyDoor)))

(fn ConstructionScript)

(fn SpawnSFX
  (params (Sound :type Sound%20Base%20Object%20Reference) (AttachToComponent :type Scene%20Component%20Object%20Reference))
  (bind _sfx (Variables|Default|GetSFX)
    (:then
      (Components|DestroyComponent _sfx))
    (:else
      _))
  (bind _returnvalue (Audio|SpawnSoundAttached Sound AttachToComponent "None" "0, 0, 0" "0, 0, 0" "KeepRelativeOffset" false 1.0 1.0 0.0 0 0))
  (Variables|Default|SetSFX _returnvalue))