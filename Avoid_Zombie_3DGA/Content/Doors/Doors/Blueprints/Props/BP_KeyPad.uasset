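; Keypad prop that lets the player enter a code to unlock a door.
; Interacting creates a WBP_Keypad widget seeded with the required code, opens it through OpenWidget, and binds to its correct-code dispatcher.
; A correct entry unbinds that dispatcher and fires the keypad's own OnUnlock dispatcher to signal the door.
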(event Custom|SendUnlockMessage
  ;[1 1 1] Unbinds the dispatcher and tells the door to unlock
  (EventDispatchers|UnbindEventfromOnCorrectCodeEntered (Variables|Default|GetKeyPadWidgetRef) (delegate Custom|SendUnlockMessage))
  (Default|CallOnUnlock))

(event EventBeginPlay)

(event Collision|EventActorBeginOverlap
  (params (OtherActor :type Actor%20Object%20Reference)))

(event EventTick
  (params (DeltaSeconds :type Float%20%28single-precision%29)))

(event EventInteract
  ;[1 1 1] Interact with key pad opens keypad widget calls global function and binds to the correct code being entered
  (bind _returnvalue (UserInterface|CreateWidget "/Game/Doors/Doors/Widgets/WBP_Keypad.WBP_Keypad_C" 0 (Utilities|Text|ToText(String) (Variables|Default|GetCode))))
  (Variables|Default|SetKeyPadWidgetRef _returnvalue)
  (CallFunction|OpenWidget (Variables|Default|GetKeyPadWidgetRef))
  (EventDispatchers|BindEventtoOnCorrectCodeEntered (Variables|Default|GetKeyPadWidgetRef) (EventDispatchers|CreateEvent :!event Custom|SendUnlockMessage)))

(fn ConstructionScript)