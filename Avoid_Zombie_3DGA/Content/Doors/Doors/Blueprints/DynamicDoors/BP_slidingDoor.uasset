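; Double sliding door that opens on interaction or is linked to a pressure plate, keypad or lever chosen by DoorType.
; BeginPlay binds to the matching prop's event; only a valid keypad sets NeedsCode, which blocks opening through Interact.
; Opening disables collision on both panels so they can slide into the wall.
; A timeline nudges each panel outward along X from its current position on every update.
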(event Custom|OpenDoor
  (bind _leftdoor (Variables|Default|GetLeftDoor))
  (bind _rightdoor (Variables|Default|GetRightDoor))
  (bind _relativelocation (Variables|/Script/Engine.SceneComponent|GetRelativeLocation _rightdoor))
  (bind _relativelocation_2 (Variables|/Script/Engine.SceneComponent|GetRelativeLocation _leftdoor))
  ;[1 1 1] Opens the doors has to disable collision to slide into the wall
  (Collision|SetCollisionEnabled (Variables|Default|GetRightDoor) "NoCollision")
  (bind _newtrack_0 (Timeline|Timeline Play)
    (:Update
      (Transformation|SetRelativeLocation _leftdoor (Math|Vector|MakeVector (Math|Float|Lerp (.x _relativelocation_2) (- (.x _relativelocation_2) 1.0) _newtrack_0) (.y _relativelocation_2) (.z _relativelocation_2)) false false)
      (Transformation|SetRelativeLocation _rightdoor (Math|Vector|MakeVector (Math|Float|Lerp (.x _relativelocation) (+ (.x _relativelocation) 1.0) _newtrack_0) (.y _relativelocation) (.z _relativelocation)) false false))))

(event EventBeginPlay
  ;[1 1 1] Gets the Enum and links the correct prop to the door
  (switch Utilities|FlowControl|Switch|SwitchonE_DoorType (Variables|Default|GetDoorType)
    (:NewEnumerator0
      (bind _unlockpressureplate (Variables|Default|GetUnlockPressurePlate)
        (:then
          (EventDispatchers|BindEventtoOnPlateDown _unlockpressureplate (EventDispatchers|CreateEvent :!event Custom|OpenDoor)))
        (:else)))
    (:NewEnumerator1
      (bind _unlockkeypad (Variables|Default|GetUnlockKeypad)
        (:then
          (EventDispatchers|BindEventtoOnUnlock _unlockkeypad (EventDispatchers|CreateEvent :!event Custom|OpenDoor))
          (Variables|Default|SetNeedsCode true))
        (:else)))
    (:NewEnumerator2
      (bind _unlocklever (Variables|Default|GetUnlockLever)
        (:then
          (EventDispatchers|BindEventtoOnLeverPulled _unlocklever (EventDispatchers|CreateEvent :!event Custom|OpenDoor)))
        (:else)))))

(event EventInteract
  (bind _leftdoor (Variables|Default|GetLeftDoor))
  (bind _rightdoor (Variables|Default|GetRightDoor))
  (bind _relativelocation (Variables|/Script/Engine.SceneComponent|GetRelativeLocation _rightdoor))
  (bind _relativelocation_2 (Variables|/Script/Engine.SceneComponent|GetRelativeLocation _leftdoor))
  ;[1 1 1] Opens the doors has to disable collision to slide into the wall
  (if (not (Variables|Default|GetNeedsCode))
    (Collision|SetCollisionEnabled (Variables|Default|GetRightDoor) "NoCollision")
    (bind _newtrack_0 (Timeline|Timeline Play)
      (:Update
        (Transformation|SetRelativeLocation _leftdoor (Math|Vector|MakeVector (Math|Float|Lerp (.x _relativelocation_2) (- (.x _relativelocation_2) 1.0) _newtrack_0) (.y _relativelocation_2) (.z _relativelocation_2)) false false)
        (Transformation|SetRelativeLocation _rightdoor (Math|Vector|MakeVector (Math|Float|Lerp (.x _relativelocation) (+ (.x _relativelocation) 1.0) _newtrack_0) (.y _relativelocation) (.z _relativelocation)) false false)))))

(fn ConstructionScript)